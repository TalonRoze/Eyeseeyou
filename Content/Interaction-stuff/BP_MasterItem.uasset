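; BP_MasterItem is an interactable item that shows a hint widget and an outline overlay material on its mesh.
; When the first-person character enters its sphere, it creates the widget, plays its pop-up animation and sets CanPressE.
; Leaving clears the outline and flag, then removes the widget after a short delay.
; The CanRecieveTrace event can also trigger the hint, with HintVisible guarding against replays.
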(event OnComponentBeginOverlap(Sphere)
  (params (OverlappedComponent :type Primitive%20Component%20Object%20Reference) (OtherActor :type Actor%20Object%20Reference) (OtherComp :type Primitive%20Component%20Object%20Reference) (OtherBodyIndex :type Integer) (bFromSweep :type Boolean) (SweepResult :type Hit%20Result%20Structure%20%28by%20ref%29))
  (Utilities|Casting|CastToBP_FirstPersonCharacter OtherActor)
  (if (Variables|Default|GetCan%20Interact)
    (bind _returnvalue (UserInterface|CreateWidget "/Game/Interaction-stuff/UI_Interact.UI_Interact_C"))
    (bind _output_get (Variables|Default|SetInteraction%20WIdget _returnvalue))
    (UserInterface|SetWidget (Variables|Default|GetWidget) _output_get)
    (Rendering|SetVisibility (Variables|Default|GetWidget) true false)
    (bind _interaction_widget (Variables|Default|GetInteraction%20WIdget)
      (:then
        (if (not (Variables|Default|GetHintVisible))
          (UserInterface|Animation|PlayAnimation _interaction_widget (Variables|/Game/Interaction-stuff/UI_Interact.UI_Interact_C|GetPopUp _interaction_widget) 0.0 1 "Forward" 1.5 false)
          (Variables|Default|SetHintVisible true)
          (Rendering|Material|SetOverlayMaterial (Variables|Default|GetStaticMesh) "/Game/Interaction-stuff/M_outline.M_outline" :!class /Script/Engine.MeshComponent)
          (Variables|Default|SetCanPressE true)))
      (:else))))

(event OnComponentEndOverlap(Sphere)
  (params (OverlappedComponent :type Primitive%20Component%20Object%20Reference) (OtherActor :type Actor%20Object%20Reference) (OtherComp :type Primitive%20Component%20Object%20Reference) (OtherBodyIndex :type Integer))
  (Utilities|Casting|CastToBP_FirstPersonCharacter OtherActor)
  (if (Variables|Default|GetCan%20Interact)
    (bind _interaction_widget (Variables|Default|GetInteraction%20WIdget)
      (:then
        (if (Variables|Default|GetHintVisible)
          (bind _returnvalue (UserInterface|Animation|PlayAnimation _interaction_widget (Variables|/Game/Interaction-stuff/UI_Interact.UI_Interact_C|GetPopUp _interaction_widget) 0.0 1 "Forward" 1.5 false))
          (Variables|Default|SetTimer _returnvalue)
          (Variables|Default|SetHintVisible false)
          (Variables|Default|SetCanPressE false)
          (Rendering|Material|SetOverlayMaterial (Variables|Default|GetStaticMesh) 0 :!class /Script/Engine.MeshComponent))
        (Utilities|FlowControl|Delay 0.15)
        (Widget|RemovefromParent (Variables|Default|GetInteraction%20WIdget))
        (Variables|Default|SetInteraction%20WIdget 0)
        (Rendering|SetVisibility (Variables|Default|GetWidget) false false))
      (:else))))

(event EventCanRecieveTrace
  (params (Can%20Interact :type Boolean))
  (if (Variables|Default|GetCan%20Interact)
    (if Can%20Interact
      (bind _interaction_widget (Variables|Default|GetInteraction%20WIdget)
        (:then
          (if (not (Variables|Default|GetHintVisible))
            (UserInterface|Animation|PlayAnimation _interaction_widget (Variables|/Game/Interaction-stuff/UI_Interact.UI_Interact_C|GetPopUp _interaction_widget) 0.0 1 "Forward" 1.5 false)
            (Variables|Default|SetHintVisible true)
            (Rendering|Material|SetOverlayMaterial (Variables|Default|GetStaticMesh) "/Game/Interaction-stuff/M_outline.M_outline" :!class /Script/Engine.MeshComponent)
            (Variables|Default|SetCanPressE true)))
        (:else
          (if (not (Variables|Default|GetHintVisible))
            (UserInterface|Animation|PlayAnimation _interaction_widget (Variables|/Game/Interaction-stuff/UI_Interact.UI_Interact_C|GetPopUp _interaction_widget) 0.0 1 "Reverse" 1.5 false)
            (Variables|Default|SetHintVisible false)
            (Rendering|Material|SetOverlayMaterial (Variables|Default|GetStaticMesh) 0 :!class /Script/Engine.MeshComponent)
            (Variables|Default|SetCanPressE false)))))))

(fn ConstructionScript)