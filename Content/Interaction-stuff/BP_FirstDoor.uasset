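; First door actor that opens by destroying itself when it receives an Interact event while in range.
; A Sphere's begin and end overlaps set and clear InDoorRange, but only when the overlapping actor casts to PlayerController.
; Interact checks that flag and prints debug messages before the destroy.
; The HasKey1 branch has no effect, so the door opens with or without the key.
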(event OnComponentBeginOverlap(Sphere)
  (params (OverlappedComponent :type Primitive%20Component%20Object%20Reference) (OtherActor :type Actor%20Object%20Reference) (OtherComp :type Primitive%20Component%20Object%20Reference) (OtherBodyIndex :type Integer) (bFromSweep :type Boolean) (SweepResult :type Hit%20Result%20Structure%20%28by%20ref%29))
  (Utilities|Casting|CastToPlayerController OtherActor)
  (Variables|Default|SetInDoorRange true))

(event OnComponentEndOverlap(Sphere)
  (params (OverlappedComponent :type Primitive%20Component%20Object%20Reference) (OtherActor :type Actor%20Object%20Reference) (OtherComp :type Primitive%20Component%20Object%20Reference) (OtherBodyIndex :type Integer))
  (Utilities|Casting|CastToPlayerController OtherActor)
  (Variables|Default|SetInDoorRange false))

(event EventInteract
  (if (Variables|Default|GetInDoorRange)
    (Development|PrintString "opening")
    (if (Variables|Default|GetHas%20Key%201)
      _
      (else
        _))
    (Development|PrintString "opening 2")
    (Actor|DestroyActor)))

(fn ConstructionScript
  (|CallParentFunction))