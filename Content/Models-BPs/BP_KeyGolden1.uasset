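; BP_KeyGolden1 is a golden key pickup that the first-person character collects with the Interact input.
; Box overlap events track whether the player is in range, and interacting there sets HasKey1 and hides the mesh.
; The actor stays in the world, and a DoOnce ensures the UI_GotKey widget is added to the viewport only once.
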(event OnComponentBeginOverlap(Box)
  (params (OverlappedComponent :type Primitive%20Component%20Object%20Reference) (OtherActor :type Actor%20Object%20Reference) (OtherComp :type Primitive%20Component%20Object%20Reference) (OtherBodyIndex :type Integer) (bFromSweep :type Boolean) (SweepResult :type Hit%20Result%20Structure%20%28by%20ref%29))
  (Utilities|Casting|CastToBP_FirstPersonCharacter OtherActor)
  (Variables|Default|SetInKeyRange true))

(event OnComponentEndOverlap(Box)
  (params (OverlappedComponent :type Primitive%20Component%20Object%20Reference) (OtherActor :type Actor%20Object%20Reference) (OtherComp :type Primitive%20Component%20Object%20Reference) (OtherBodyIndex :type Integer))
  (Utilities|Casting|CastToBP_FirstPersonCharacter OtherActor)
  (Variables|Default|SetInKeyRange false))

(event Input|EnhancedActionEvents|EnhancedInputActionIA_Interact
  (params (ActionValue :type Boolean) (ElapsedSeconds :type Float%20%28double-precision%29) (TriggeredSeconds :type Float%20%28double-precision%29) (InputAction :type Input%20Action%20Object%20Reference :default "/Game/Interaction-stuff/IA_Interact.IA_Interact"))
  (if (Variables|Default|GetInKeyRange)
    (Variables|Default|SetHasKey1 true)
    (Rendering|SetVisibility (Variables|Default|GetStaticMesh) false false)
    (Utilities|FlowControl|DoOnce false
      (:Completed
        (bind _returnvalue (UserInterface|CreateWidget "/Game/UI/UI_GotKey.UI_GotKey_C"))
        (bind _output_get (Variables|Default|SetNewVar _returnvalue))
        (UserInterface|Viewport|AddtoViewport _output_get 0)))))

(fn ConstructionScript)