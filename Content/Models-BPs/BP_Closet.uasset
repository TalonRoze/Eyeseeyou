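; BP_Closet is a closet actor that the first-person character can step into and out of.
; A Box overlap with BP_FirstPersonCharacter sets InRange, which gates the IA_Interact input.
; Each interaction toggles InCloset and teleports the character taken from the overlap, either onto the mesh's location or to a small fixed world-space Y offset from it when leaving.
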(event OnComponentEndOverlap(Box)
  (params (OverlappedComponent :type Primitive%20Component%20Object%20Reference) (OtherActor :type Actor%20Object%20Reference) (OtherComp :type Primitive%20Component%20Object%20Reference) (OtherBodyIndex :type Integer))
  (Utilities|Casting|CastToBP_FirstPersonCharacter OtherActor)
  (Variables|Default|SetInRange false))

(event OnComponentBeginOverlap(Box)
  (params (OverlappedComponent :type Primitive%20Component%20Object%20Reference) (OtherActor :type Actor%20Object%20Reference) (OtherComp :type Primitive%20Component%20Object%20Reference) (OtherBodyIndex :type Integer) (bFromSweep :type Boolean) (SweepResult :type Hit%20Result%20Structure%20%28by%20ref%29))
  (Utilities|Casting|CastToBP_FirstPersonCharacter OtherActor)
  (Variables|Default|SetInRange true))

(event Input|EnhancedActionEvents|EnhancedInputActionIA_Interact
  (params (ActionValue :type Boolean) (ElapsedSeconds :type Float%20%28double-precision%29) (TriggeredSeconds :type Float%20%28double-precision%29) (InputAction :type Input%20Action%20Object%20Reference :default "/Game/Interaction-stuff/IA_Interact.IA_Interact"))
  (if (Variables|Default|GetInRange)
    (if (Variables|Default|GetInCloset)
      (bind _asbp_first_person_character (Utilities|Casting|CastToBP_FirstPersonCharacter (stale OnComponentBeginOverlap(Box) OtherActor)))
      (Transformation|SetActorLocationAndRotation _asbp_first_person_character (+ (Transformation|GetWorldLocation (Variables|Default|GetStaticMesh)) "0.000000,-10.000000,0.000000"))
      (Variables|Default|SetInCloset false)
      (else
        (bind _asbp_first_person_character_2 (Utilities|Casting|CastToBP_FirstPersonCharacter (stale OnComponentBeginOverlap(Box) OtherActor)))
        (Transformation|SetActorLocationAndRotation _asbp_first_person_character_2 (Transformation|GetWorldLocation (Variables|Default|GetStaticMesh)))
        (Variables|Default|SetInCloset true)))))

(fn ConstructionScript)