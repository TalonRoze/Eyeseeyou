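; BP_DoorV2 is a locked door that the player opens by interacting while in range with the golden key collected.
; A Box overlap with BP_FirstPersonCharacter toggles InDoorRange.
; On the IA_Interact input, it looks up the BP_KeyGolden1 actor and checks its HasKey1 flag, then destroys the door if set.
; The key state lives on the key actor rather than the player.
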(event OnComponentBeginOverlap(Box)
  (params (OverlappedComponent :type Primitive%20Component%20Object%20Reference) (OtherActor :type Actor%20Object%20Reference) (OtherComp :type Primitive%20Component%20Object%20Reference) (OtherBodyIndex :type Integer) (bFromSweep :type Boolean) (SweepResult :type Hit%20Result%20Structure%20%28by%20ref%29))
  (Utilities|Casting|CastToBP_FirstPersonCharacter OtherActor)
  (Variables|Default|SetInDoorRange true))

(event OnComponentEndOverlap(Box)
  (params (OverlappedComponent :type Primitive%20Component%20Object%20Reference) (OtherActor :type Actor%20Object%20Reference) (OtherComp :type Primitive%20Component%20Object%20Reference) (OtherBodyIndex :type Integer))
  (Utilities|Casting|CastToBP_FirstPersonCharacter OtherActor)
  (Variables|Default|SetInDoorRange false))

(event Input|EnhancedActionEvents|EnhancedInputActionIA_Interact
  (params (ActionValue :type Boolean) (ElapsedSeconds :type Float%20%28double-precision%29) (TriggeredSeconds :type Float%20%28double-precision%29) (InputAction :type Input%20Action%20Object%20Reference :default "/Game/Interaction-stuff/IA_Interact.IA_Interact"))
  (if (Variables|Default|GetInDoorRange)
    (bind _returnvalue (Actor|GetActorOfClass "/Game/Models-BPs/BP_KeyGolden1.BP_KeyGolden1_C"))
    (if (Variables|/Game/Models-BPs/BP_KeyGolden1.BP_KeyGolden1_C|GetHasKey1 _returnvalue)
      (Actor|DestroyActor))))

(fn ConstructionScript)

(fn NewFunction)